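; BP_SoundWaveRing is a one-shot effect actor that shows an expanding sound wave ring.
; On BeginPlay it creates a dynamic material instance of MI_SoundWaveRing on RingMesh and plays WaveTimeline.
; Timeline progress is remapped to drive both the ring's uniform world scale and the material's Exp parameter as they grow.
; The actor destroys itself when the timeline finishes.
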(event `self.ReceiveBeginPlay`
  (bind _returnvalue (`PrimitiveComponent.CreateDynamicMaterialInstance` (`self.RingMesh`) 0 "/Game/Effects/MI_SoundWaveRing.MI_SoundWaveRing" "None"))
  (set `self.DynamicMat` _returnvalue)
  (bind (_direction _progress) (`Timeline|WaveTimeline`)
    (:`Update`
      (bind _returnvalue_2 (`KismetMathLibrary.MapRangeClamped` _progress 0.0 1.0 0.1 6.0))
      (`MaterialInstanceDynamic.SetScalarParameterValue` (`self.DynamicMat`) "Exp" _returnvalue_2)
      (`SceneComponent.SetWorldScale3D` (`self.RingMesh`) (`KismetMathLibrary.Conv_DoubleToVector` _returnvalue_2)))
    (:`Finished`
      (`self.K2_DestroyActor`))))

(fn `UserConstructionScript`)