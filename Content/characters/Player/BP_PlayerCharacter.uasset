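; Player character Blueprint that handles camera look and zoom, movement, and an attack montage.
; Enhanced Input actions drive camera rotation and inverted zoom, while legacy axis events store forward/right values that Tick passes to SetMovementInput.
; Tick also polls W, S, A and D directly in a priority chain, forcing single-direction movement relative to control yaw.
; PlayAttackAnimation plays AM_Attack on the mesh's anim instance.
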(event `EnhancedInput|/Game/Input/Actions/IA_CameraLook`
  (params (ActionValue :type "Vector2D Structure") (ElapsedSeconds :type "Float (double-precision)") (TriggeredSeconds :type "Float (double-precision)") (InputAction :type "InputAction Object Reference" :default "/Game/Input/Actions/IA_CameraLook.IA_CameraLook"))
  (bind (_x _y) (`KismetMathLibrary.BreakVector2D` ActionValue))
  ; camera视角旋转
  (:`Triggered`
    (`self.AddCameraRotation` _x _y)))

(event `EnhancedInput|/Game/Input/Actions/IA_Zoom`
  (params (ActionValue :type "Float (double-precision)") (ElapsedSeconds :type "Float (double-precision)") (TriggeredSeconds :type "Float (double-precision)") (InputAction :type "InputAction Object Reference" :default "/Game/Input/Actions/IA_Zoom.IA_Zoom"))
  ; 视角拉远/近
  (:`Triggered`
    (`self.ZoomCamera` (* ActionValue -1.0))))

(event `InputAxis|MoveForward`
  (params (AxisValue :type "Float (single-precision)"))
  ; 强行输入移动
  (set `self.ForwardInput` AxisValue))

(event `InputAxis|MoveRight`
  (params (AxisValue :type "Float (single-precision)"))
  ; 强行输入移动
  (set `self.RightInput` AxisValue))

(event `self.ReceiveTick`
  (params (DeltaSeconds :type "Float (single-precision)"))
  (bind _returnvalue (`KismetMathLibrary.MakeRotator` 0.0 0.0 (.yaw (`self.GetControlRotation` (`GameplayStatics.GetPlayerPawn` 0)))))
  (bind _returnvalue_2 (`KismetMathLibrary.GetForwardVector` _returnvalue))
  (bind _returnvalue_3 (`KismetMathLibrary.GetRightVector` _returnvalue))
  ; 强行输入移动
  (`self.SetMovementInput` (`self.ForwardInput`) (`self.RightInput`))
  (if (`PlayerController.IsInputKeyDown` (`GameplayStatics.GetPlayerController` 0) "W")
    (`self.AddMovementInput` _returnvalue_2)
    (elif (`PlayerController.IsInputKeyDown` (`GameplayStatics.GetPlayerController` 0) "S")
      (`self.AddMovementInput` _returnvalue_2 -1.0)
      (elif (`PlayerController.IsInputKeyDown` (`GameplayStatics.GetPlayerController` 0) "A")
        (`self.AddMovementInput` _returnvalue_3 -1.0)
        (elif (`PlayerController.IsInputKeyDown` (`GameplayStatics.GetPlayerController` 0) "D")
          (`self.AddMovementInput` _returnvalue_3))))))

(fn `Get Control Rotation`)

(fn `PlayAttackAnimation`
  (`AnimInstance.Montage_Play` (`SkeletalMeshComponent.GetAnimInstance` (`self.Mesh`)) "/Game/characters/Player/Attack/AM_Attack.AM_Attack" 1.0 "MontageLength" 0.0 true))

(fn `UserConstructionScript`)